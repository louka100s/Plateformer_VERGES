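; BP_Door is an interactable door that swings open and closed on alternate Interact events.
; A FlipFlop plays or reverses DoorTimeline, whose track drives the door mesh's yaw through a Lerp.
; Overlapping the Box adds a W_Interact prompt to the viewport with no actor filter.
; The prompt has no end-overlap removal; timeline updates clear all W_Interact widgets instead.
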(event `/Game/Game/BP/I_Interact.Interact`
  (`/Engine/EditorBlueprintResources/StandardMacros.FlipFlop`
    (:`A`
      (bind (_direction _door_track) (`Timeline|Door Timeline` :!label _label)
        (:`Update`
          (`SceneComponent.K2_SetRelativeRotation` (`self.Mesh_Door`) (`KismetMathLibrary.MakeRotator` 0.0 0.0 (`KismetMathLibrary.Lerp` 0.0 380.0 _door_track)) false false)
          (bind _foundwidgets (`WidgetBlueprintLibrary.GetAllWidgetsOfClass` "/Game/Game/BP/W_Interact.W_Interact_C"))
          (`Widget.RemoveFromParent` _foundwidgets))))
    (:`B`
      (goto _label :!via `Reverse`))))

(event `self.Box.OnComponentBeginOverlap`
  (params (OverlappedComponent :type "PrimitiveComponent Object Reference") (OtherActor :type "Actor Object Reference") (OtherComp :type "PrimitiveComponent Object Reference") (OtherBodyIndex :type Integer) (bFromSweep :type Boolean) (SweepResult :type "HitResult Structure (by ref)"))
  (bind _returnvalue (`|CreateWidget` "/Game/Game/BP/W_Interact.W_Interact_C" (`GameplayStatics.GetPlayerController` 0)))
  (`UserWidget.AddToViewport` _returnvalue 0))

(fn `UserConstructionScript`)