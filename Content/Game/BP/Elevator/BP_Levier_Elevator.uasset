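; Elevator lever Blueprint that flags the lever as activated in the game instance when the player interacts with it.
; On BeginPlay it caches the BP_GameInstance, and Interact sets its LevierState to true and prints a debug message.
; The first overlap of the lever's collision box creates an interaction prompt widget and adds it to the viewport, with no logic to remove it.
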(event `self.ReceiveBeginPlay`
  (bind _asbp_game_instance (cast `/Game/Game/BP/BP_GameInstance` (`GameplayStatics.GetGameInstance`)))
  (set `self.As BP Game Instance` _asbp_game_instance))

(event `/Game/Game/BP/I_Interact.Interact`
  (set `/Game/Game/BP/BP_GameInstance.LevierState` true (`self.As BP Game Instance`))
  (`KismetSystemLibrary.PrintString` "Hello"))

(event `self.LevierBoxCollision.OnComponentBeginOverlap`
  (params (OverlappedComponent :type "PrimitiveComponent Object Reference") (OtherActor :type "Actor Object Reference") (OtherComp :type "PrimitiveComponent Object Reference") (OtherBodyIndex :type Integer) (bFromSweep :type Boolean) (SweepResult :type "HitResult Structure (by ref)"))
  (`/Engine/EditorBlueprintResources/StandardMacros.DoOnce` false
    (:`Completed`
      (bind _returnvalue (`|CreateWidget` "/Game/Game/BP/W_Interact.W_Interact_C" (`GameplayStatics.GetPlayerController` 0)))
      (`UserWidget.AddToViewport` _returnvalue 0))))

(fn `UserConstructionScript`)