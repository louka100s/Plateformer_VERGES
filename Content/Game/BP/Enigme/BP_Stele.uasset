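; BP_Stele is a puzzle actor whose stele moves between a lowered and a raised position according to the light puzzle state.
; On BeginPlay it caches BP_GameInstance and binds to its OnLightToggle event.
; Each toggle queries GetSteleState and instantly snaps the Stele component's relative location up or back to its origin, with no interpolation or sweep.
; The position is not synced on BeginPlay, only when the event fires.
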(event `self.ReceiveBeginPlay`
  (bind _asbp_game_instance (cast `/Game/Game/BP/BP_GameInstance` (`GameplayStatics.GetGameInstance`)))
  (bind _output_get (set `self.As BP Game Instance` _asbp_game_instance))
  (add `/Game/Game/BP/BP_GameInstance.OnLightToggle` _output_get (delegate `UpdateSteleState`)))

(event `UpdateSteleState`
  (bind _stelestate (`/Game/Game/BP/BP_GameInstance.GetSteleState` (`self.As BP Game Instance`)))
  (if _stelestate
    (`SceneComponent.K2_SetRelativeLocation` (`self.Stele`) (0.0 0.0 200.0) false false)
    (else
      (`SceneComponent.K2_SetRelativeLocation` (`self.Stele`) (0.0 0.0 0.0) false false))))

(fn `UserConstructionScript`)