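; BP_Light is a numbered point light whose visibility follows a light state held in BP_GameInstance.
; UpdateLight looks up the state for its Number on the game instance and applies it to the PointLight component.
; BeginPlay calls UpdateLight before the game instance reference is assigned, then caches it and binds UpdateLight to OnLightToggle for later changes.
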(event `self.ReceiveBeginPlay`
  (`self.UpdateLight`)
  (bind _asbp_game_instance (cast `/Game/Game/BP/BP_GameInstance` (`GameplayStatics.GetGameInstance`)))
  (bind _output_get (set `self.As BP Game Instance` _asbp_game_instance))
  (add `/Game/Game/BP/BP_GameInstance.OnLightToggle` _output_get (delegate `UpdateLight`)))

(event `UpdateLight`
  (bind _light_state (`/Game/Game/BP/BP_GameInstance.GetLightStateByNumber` (`self.As BP Game Instance`) (`self.Number`)))
  (`SceneComponent.SetVisibility` (`self.PointLight`) _light_state false))

(fn `UserConstructionScript`)