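; BP_BigGate is a large gate actor that players open and close through an Interact event.
; A FlipFlop alternates between playing and reversing a Timeline that lerps the gate mesh's relative Z to raise or lower it.
; The first overlap with the gate's collision shows a W_Interact prompt through a DoOnce, with no actor filter.
; Timeline updates remove W_Interact widgets from the viewport.
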(event `/Game/Game/BP/I_Interact.Interact`
  (`/Engine/EditorBlueprintResources/StandardMacros.FlipFlop`
    (:`A`
      (bind (_direction _door_track) (`Timeline|Timeline` :!label _label)
        (:`Update`
          (`SceneComponent.K2_SetRelativeLocation` (`self.Gate`) (`KismetMathLibrary.MakeVector` 0.0 0.0 (`KismetMathLibrary.Lerp` 0.0 1000.0 _door_track)) false false)
          (bind _foundwidgets (`WidgetBlueprintLibrary.GetAllWidgetsOfClass` "/Game/Game/BP/W_Interact.W_Interact_C"))
          (`Widget.RemoveFromParent` _foundwidgets))))
    (:`B`
      (goto _label :!via `Reverse`))))

(event `self.Gatecollision.OnComponentBeginOverlap`
  (params (OverlappedComponent :type "PrimitiveComponent Object Reference") (OtherActor :type "Actor Object Reference") (OtherComp :type "PrimitiveComponent Object Reference") (OtherBodyIndex :type Integer) (bFromSweep :type Boolean) (SweepResult :type "HitResult Structure (by ref)"))
  (`/Engine/EditorBlueprintResources/StandardMacros.DoOnce` false
    (:`Completed`
      (bind _returnvalue (`|CreateWidget` "/Game/Game/BP/W_Interact.W_Interact_C"))
      (`UserWidget.AddToViewport` _returnvalue 0))))

(fn `UserConstructionScript`)