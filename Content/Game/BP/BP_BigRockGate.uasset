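; BP_BigRockGate is a gate that rises when interacted with, provided the player's score is high enough.
; The first overlap with its collision shows a W_Interact prompt, only once thanks to a DoOnce.
; Interact checks Score on BP_GameInstance against a threshold, then plays a Timeline that lerps the Gate's relative height.
; Each Timeline update also removes the W_Interact widgets from screen.
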(event `self.ReceiveBeginPlay`
  (bind _asbp_game_instance (cast `/Game/Game/BP/BP_GameInstance` (`GameplayStatics.GetGameInstance`)))
  (set `self.As BP Game Instance` _asbp_game_instance))

(event `self.Interact`
  (`KismetSystemLibrary.PrintString` "OUI CA MARCHE" false true (struct :`R` 1.0 :`B` 0.425569 :`A` 1.0))
  (if (>= (`/Game/Game/BP/BP_GameInstance.Score` (`self.As BP Game Instance`)) 5)
    (bind (_direction _door_track) (`Timeline|Timeline`)
      (:`Update`
        (`SceneComponent.K2_SetRelativeLocation` (`self.Gate`) (`KismetMathLibrary.MakeVector` 0.0 0.0 (`KismetMathLibrary.Lerp` 0.0 1000.0 _door_track)) false false)
        (bind _foundwidgets (`WidgetBlueprintLibrary.GetAllWidgetsOfClass` "/Game/Game/BP/W_Interact.W_Interact_C"))
        (`Widget.RemoveFromParent` _foundwidgets)))))

(event `self.Gatecollision.OnComponentBeginOverlap`
  (params (OverlappedComponent :type "PrimitiveComponent Object Reference") (OtherActor :type "Actor Object Reference") (OtherComp :type "PrimitiveComponent Object Reference") (OtherBodyIndex :type Integer) (bFromSweep :type Boolean) (SweepResult :type "HitResult Structure (by ref)"))
  (`/Engine/EditorBlueprintResources/StandardMacros.DoOnce` false
    (:`Completed`
      (bind _returnvalue (`|CreateWidget` "/Game/Game/BP/W_Interact.W_Interact_C"))
      (`UserWidget.AddToViewport` _returnvalue 0))))

(fn `UserConstructionScript`)